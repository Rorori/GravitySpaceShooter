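; Scrolling background actor that loops two sprites downward to create an endless vertical scroll.
; Each Tick moves both sprites down in relative Z by UnitsPerSecond scaled by delta time, keeping the speed frame-rate independent.
; After each move, a sprite that falls below ResetLocation's Z is raised by twice SpriteHeight to sit above the other and descend again.
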(event `self.ReceiveBeginPlay`)

(event `self.ReceiveActorBeginOverlap`
  (params (OtherActor :type "Actor Object Reference")))

(event `self.ReceiveTick`
  (params (DeltaSeconds :type "Float (single-precision)"))
  (bind _returnvalue (* DeltaSeconds (`self.UnitsPerSecond`)))
  ;[1 1 1] Move both sprites
  (`self.MoveSprite` _returnvalue (`self.Sprite1`)) ; Move sprite 1
  (`self.MoveSprite` _returnvalue (`self.Sprite2`)) ; Move sprite 2
)

(fn `CheckAndResetSprite`
  (params (Sprite :type "PaperSpriteComponent Object Reference") (SpriteLocation :type "Vector Structure"))
  (bind _z (.z SpriteLocation))
  ;[1 1 1] Check if sprite is below reset location. If so, it is out of sight. Move it above the other sprite.
  (if (< _z (.z (`self.ResetLocation`)))
    (`SceneComponent.K2_SetRelativeLocation` Sprite (`KismetMathLibrary.MakeVector` (.x SpriteLocation) (.y SpriteLocation) (+ _z (* (`self.SpriteHeight`) 2.0))) false false) ; Move sprite up and let it descend again
  ))

(fn `MoveSprite`
  (params (UnitsToMove :type "Float (double-precision)") (SpriteToMove :type "PaperSpriteComponent Object Reference"))
  (bind _returnvalue (`KismetMathLibrary.MakeVector` (.x (`SceneComponent.RelativeLocation` SpriteToMove)) (.y (`SceneComponent.RelativeLocation` SpriteToMove)) (- (.z (`SceneComponent.RelativeLocation` SpriteToMove)) UnitsToMove)))
  ;[1 1 1] Move Sprite down vertically by given number of units
  (`SceneComponent.K2_SetRelativeLocation` SpriteToMove _returnvalue false false)
  (`self.CheckAndResetSprite` SpriteToMove _returnvalue) ; Check if the sprite's new position places it out of sight. If so, move it above the other sprite.
)

(fn `UserConstructionScript`)