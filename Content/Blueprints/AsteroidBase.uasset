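; Base asteroid actor for a Paper2D game, with a randomly chosen look and spin.
; The construction script picks a random sprite from AsteroidSpriteArray, and BeginPlay gives RotatingMovement a random pitch rate within the min/max range.
; SetVelocity sets the ProjectileMovement velocity to move the asteroid.
; BeginPlay also queries all ExplodingAsteroid actors without using the result, then increments AsteroidDestroyCount.
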(event `self.ReceiveBeginPlay`
  ;[1 1 1] Set the asteroid rotating in a random direction at a random rate
  (set `RotatingMovementComponent.RotationRate` (`KismetMathLibrary.MakeRotator` 0.0 (`KismetMathLibrary.RandomFloatInRange` (`self.MinRotationRate`) (`self.MaxRotationRate`))) (`self.RotatingMovement`))
  (`GameplayStatics.GetAllActorsOfClass` "/Game/Blueprints/ExplodingAsteroid.ExplodingAsteroid_C")
  (bind _result (`/Engine/EditorBlueprintResources/StandardMacros.IncrementFloat` (`self.AsteroidDestroyCount`))
    (:`  `
      (set `self.AsteroidDestroyCount` _result))))

(event `self.ReceiveActorBeginOverlap`
  (params (OtherActor :type "Actor Object Reference")))

(event `self.ReceiveTick`
  (params (DeltaSeconds :type "Float (single-precision)")))

(fn `SetVelocity`
  (params (NewVelocity :type "Vector Structure"))
  ;[1 1 1] Make the asteroid move
  (set `MovementComponent.Velocity` NewVelocity (`self.ProjectileMovement`)))

(fn `UserConstructionScript`
  (bind _asteroidspritearray (`self.AsteroidSpriteArray`))
  ;[1 1 1] Pick a random sprite for the asteroid object
  (`PaperSpriteComponent.SetSprite` (`self.AsteroidSprite`) (`KismetArrayLibrary.Array_Get` _asteroidspritearray (`KismetMathLibrary.RandomIntegerInRange` 0 (- (`KismetArrayLibrary.Array_Length` _asteroidspritearray) 1)))))