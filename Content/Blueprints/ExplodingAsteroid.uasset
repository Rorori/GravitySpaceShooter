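; Exploding asteroid actor that breaks into smaller fragments when another actor, intended to be a projectile, overlaps it.
; On overlap it reports to the player ship's asteroid counter, destroys the overlapping actor without checking its type, spawns debris and destroys itself.
; SpawnDebris runs three times, each creating an AsteroidFragment at the asteroid's transform with a random direction scaled by DebrisSpeed.
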(event `self.ReceiveBeginPlay`
  (`parent.ReceiveBeginPlay`))

(event `self.ReceiveActorBeginOverlap`
  (params (OtherActor :type "Actor Object Reference"))
  (bind _asplayer_ship_character_2 (cast `/Game/Blueprints/Blueprints/PlayerShipCharacter2` (`GameplayStatics.GetPlayerCharacter` 0)))
  (`/Game/Blueprints/Blueprints/PlayerShipCharacter2.AsteroidCounter` _asplayer_ship_character_2 1)
  (`self.K2_DestroyActor` OtherActor) ; destroy projectile
  (`self.SpawnDebris` (`KismetMathLibrary.RandomUnitVector`))
  (`self.SpawnDebris` (`KismetMathLibrary.RandomUnitVector`)) ; Create fragment moving northwest
  (`self.SpawnDebris` (`KismetMathLibrary.RandomUnitVector`)) ; Create fragment moving northeast
  (`self.K2_DestroyActor`))

(event `self.ReceiveTick`
  (params (DeltaSeconds :type "Float (single-precision)")))

(fn `SpawnDebris`
  (params (Velocity :type "Vector Structure"))
  ;[1 1 1] Spawn an asteroid fragment and set it moving in a given direction
  (bind _returnvalue (`|SpawnActorFromClass` "/Game/Blueprints/AsteroidFragment.AsteroidFragment_C" (`self.GetTransform`) "Undefined" "OverrideRootScale"))
  (`self.SetVelocity` _returnvalue (* Velocity (`self.DebrisSpeed`))))

(fn `UserConstructionScript`
  (`parent.UserConstructionScript`))