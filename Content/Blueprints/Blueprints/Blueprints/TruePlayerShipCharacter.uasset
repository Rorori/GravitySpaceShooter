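; Player ship Character that flies on the X/Z axes, fires photon torpedoes and restarts the level when hit by an asteroid.
; Axis inputs add velocity-change impulses, and horizontal input also sets control and actor pitch.
; Fire spawns a PhotonTorpedo at the ship's location with velocity along its forward vector.
; An asteroid capsule hit hides the ship, destroys the asteroid, then reopens the level cached at BeginPlay after a delay.
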(event `self.CapsuleComponent.OnComponentHit`
  (params (OtherActor :type "Actor Object Reference") (OtherComp :type "PrimitiveComponent Object Reference") (NormalImpulse :type "Vector Structure") (Hit :type "HitResult Structure (by ref)"))
  ;[1 1 1] Restart the level when an asteroid hits the player
  (bind _asasteroid_base (cast `/Game/Blueprints/AsteroidBase` OtherActor))
  (`self.SetActorHiddenInGame` true)
  (`self.K2_DestroyActor` _asasteroid_base)
  (`KismetSystemLibrary.Delay` 2.0)
  (`GameplayStatics.OpenLevel` (`self.CurrentLevelName`)))

(event `self.ReceiveBeginPlay`
  ;[1 1 1] Rotate actor to point up when playing
  (bind _returnvalue (`GameplayStatics.GetCurrentLevelName` true))
  (set `self.CurrentLevelName` (`KismetStringLibrary.Conv_StringToName` _returnvalue)))

(event `/Game/Blueprints/PlayerShipCharacter.ReceiveActorBeginOverlap`
  (params (OtherActor :type "Actor Object Reference")))

(event `InputAxis|MoveRight`
  (params (AxisValue :type "Float (single-precision)"))
  (bind _controlrotationvalue (`self.ControlRotationValue`))
  ;[1 1 1] HAndle horizontal and vertical movement
  (set `self.FireBackwards` AxisValue)
  (`PrimitiveComponent.AddImpulse` (`MovementComponent.UpdatedPrimitive` (`self.CharacterMovement`)) (`KismetMathLibrary.MakeVector` (* 10.0 AxisValue)) "None" true)
  (set `self.ControlRotationValue` (`KismetMathLibrary.MakeRotator` 0.0 (* 90.0 (stale `InputAxis|MoveUp` AxisValue))))
  (`Controller.SetControlRotation` (`GameplayStatics.GetPlayerController` 0) _controlrotationvalue)
  (`self.SetActorRotation` _controlrotationvalue))

(event `self.ReceiveTick`
  (params (DeltaSeconds :type "Float (single-precision)")))

(event `InputAxis|MoveUp`
  (params (AxisValue :type "Float (single-precision)"))
  ;[1 1 1] HAndle horizontal and vertical movement
  (`PrimitiveComponent.AddImpulse` (`MovementComponent.UpdatedPrimitive` (`self.CharacterMovement`)) (`KismetMathLibrary.MakeVector` 0.0 0.0 (* 10.0 AxisValue)) "None" true))

(event `InputAction|Fire`
  (params (Key :type "Key Structure" :default "AnyKey"))
  (bind _returnvalue (`self.GetActorForwardVector`))
  ;[1 1 1] Fire a Photon Torpedo
  (:`Pressed`
    (bind _returnvalue_2 (`|SpawnActorFromClass` "/Game/Blueprints/PhotonTorpedo.PhotonTorpedo_C" (`KismetMathLibrary.MakeTransform` (+ (* _returnvalue 0.0) (`self.K2_GetActorLocation`)) (struct)) "Undefined" "OverrideRootScale"))
    (`/Game/Blueprints/PhotonTorpedo.SetVelocity` _returnvalue_2 (* _returnvalue (`self.TorpedoSpeed`)))))

(event `self.ArrowComponent.OnEndCursorOver`
  (params (TouchedComponent :type "PrimitiveComponent Object Reference")))

(fn `UserConstructionScript`)