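; Player 1's ship in a two-player asteroid shooter on the XZ plane, also relaying Player 2's input to PlayerShipCharacter3.
; Axis input sets rotation, while Tick adds velocity impulses combining input with a distance-scaled pull toward the other ship.
; Fire launches a PhotonTorpedo along the ship's forward vector.
; Torpedo or asteroid contact hides the ship and reloads the level after a delay; helper functions track asteroid score.
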(event `self.ReceiveActorBeginOverlap`
  (params (OtherActor :type "Actor Object Reference")))

(event `self.CapsuleComponent.OnComponentBeginOverlap`
  (params (OtherActor :type "Actor Object Reference") (OtherComp :type "PrimitiveComponent Object Reference") (OtherBodyIndex :type Integer) (bFromSweep :type Boolean) (SweepResult :type "HitResult Structure (by ref)"))
  ;[1 1 1] Restart the level when a torpedo hits the player
  (bind _asphoton_torpedo (cast `/Game/Blueprints/PhotonTorpedo` OtherActor))
  (`self.SetActorHiddenInGame` true)
  (`self.K2_DestroyActor` _asphoton_torpedo)
  (`KismetSystemLibrary.Delay` 2.0)
  (`GameplayStatics.OpenLevel` (`self.CurrentLevelName`)))

(event `self.CapsuleComponent.OnComponentHit`
  (params (OtherActor :type "Actor Object Reference") (OtherComp :type "PrimitiveComponent Object Reference") (NormalImpulse :type "Vector Structure") (Hit :type "HitResult Structure (by ref)"))
  ;[1 1 1] Restart the level when an asteroid hits the player
  (bind _asasteroid_base (cast `/Game/Blueprints/AsteroidBase` OtherActor))
  (`self.SetActorHiddenInGame` true)
  (`self.K2_DestroyActor` _asasteroid_base)
  (`KismetSystemLibrary.Delay` 2.0)
  (`GameplayStatics.OpenLevel` (`self.CurrentLevelName`)))

(event `self.ReceiveBeginPlay`
  (`PrimitiveComponent.AddImpulse` (`MovementComponent.UpdatedPrimitive` (`self.CharacterMovement`)) (* (`KismetMathLibrary.MakeVector` 0.0 0.0 (`KismetMathLibrary.RandomFloatInRange` -1.0 1.0)) 500.0) "None" false)
  (bind _returnvalue (`GameplayStatics.GetCurrentLevelName` true))
  (set `self.CurrentLevelName` (`KismetStringLibrary.Conv_StringToName` _returnvalue)))

(event `InputAxis|MoveRightPlayer1` :consume false
  (params (AxisValue :type "Float (single-precision)"))
  (bind _returnvalue (* AxisValue -90.0))
  ;[1 1 1] Movement
  (`PrimitiveComponent.AddImpulse` (`MovementComponent.UpdatedPrimitive` (`self.CharacterMovement`)) (0.0 0.0 0.0) "None" true)
  (if (> (`KismetMathLibrary.Abs` _returnvalue) 45.0)
    (set `self.ControlShipRotation` (`KismetMathLibrary.MakeRotator` 0.0 (+ _returnvalue 90.0)))))

(event `InputAxis|MoveRightPlayer2`
  (params (AxisValue :type "Float (single-precision)"))
  ;[1 1 1] Player 2 controls
  (bind _asplayer_ship_character_3 (cast `/Game/Blueprints/Blueprints/PlayerShipCharacter3` (`GameplayStatics.GetPlayerCharacter` 1)))
  (`/Game/Blueprints/Blueprints/PlayerShipCharacter3.MoveRight` _asplayer_ship_character_3 AxisValue))

(event `MoveRightPlayer1`
  (params (AxisValue :type "Float (double-precision)")))

(event `self.ReceiveTick`
  (params (DeltaSeconds :type "Float (single-precision)"))
  ;[1 1 1] Movement
  (`self.SetActorRotation` (`self.ControlShipRotation`))
  (`PrimitiveComponent.AddImpulse` (`MovementComponent.UpdatedPrimitive` (`self.CharacterMovement`)) (`KismetMathLibrary.MakeVector` (+ (* 10.0 (stale `InputAxis|MoveRightPlayer1` AxisValue)) (* (- (.x (`self.K2_GetActorLocation`)) (.x (`self.K2_GetActorLocation` (`GameplayStatics.GetPlayerCharacter` 1)))) -0.03)) 0.0 (+ (* 10.0 (stale `InputAxis|MoveUpPLayer1` AxisValue)) (* (- (.z (`self.K2_GetActorLocation`)) (.z (`self.K2_GetActorLocation` (`GameplayStatics.GetPlayerCharacter` 1)))) -0.03))) "None" true))

(event `MoveUpPlayer1`
  (params (AxisValue :type "Float (double-precision)")))

(event `InputAxis|MoveUpPLayer1` :consume false
  (params (AxisValue :type "Float (single-precision)"))
  (bind _returnvalue (* AxisValue 90.0))
  ;[1 1 1] Movement
  (`PrimitiveComponent.AddImpulse` (`MovementComponent.UpdatedPrimitive` (`self.CharacterMovement`)) (0.0 0.0 0.0) "None" true)
  (if (> (`KismetMathLibrary.Abs` _returnvalue) 45.0)
    (set `self.ControlShipRotation` (`KismetMathLibrary.MakeRotator` 0.0 _returnvalue))))

(event `InputAxis|MoveUpPlayer2`
  (params (AxisValue :type "Float (single-precision)"))
  ;[1 1 1] Player 2 controls
  (bind _asplayer_ship_character_3 (cast `/Game/Blueprints/Blueprints/PlayerShipCharacter3` (`GameplayStatics.GetPlayerCharacter` 1)))
  (`/Game/Blueprints/Blueprints/PlayerShipCharacter3.MoveUp` _asplayer_ship_character_3 AxisValue))

(event `InputAction|FirePlayer2`
  (params (Key :type "Key Structure" :default "AnyKey"))
  ;[1 1 1] Player 2 controls
  (:`Pressed`
    (bind _asplayer_ship_character_3 (cast `/Game/Blueprints/Blueprints/PlayerShipCharacter3` (`GameplayStatics.GetPlayerCharacter` 1)))
    (`/Game/Blueprints/Blueprints/PlayerShipCharacter3.FirePlayer2` _asplayer_ship_character_3)))

(event `InputAction|FirePlayer1`
  (params (Key :type "Key Structure" :default "AnyKey"))
  (bind _returnvalue (`self.GetActorForwardVector`))
  ;[1 1 1] Fire a Photon Torpedo
  (:`Pressed`
    (bind _returnvalue_2 (`|SpawnActorFromClass` "/Game/Blueprints/PhotonTorpedo.PhotonTorpedo_C" (`KismetMathLibrary.MakeTransform` (+ (* _returnvalue 75.0) (`self.K2_GetActorLocation`)) (`KismetMathLibrary.MakeRotator` 0.0 (+ (.pitch (`self.ControlShipRotation`)) -90.0))) "Undefined" "OverrideRootScale"))
    (`/Game/Blueprints/PhotonTorpedo.SetVelocity` _returnvalue_2 (* _returnvalue (`self.TorpedoSpeed`)))))

(event `Key|Escape`
  (params (Key :type "Key Structure" :default "AnyKey"))
  ;[1 1 1] Quit Game
  (:`Pressed`
    (`KismetSystemLibrary.QuitGame` null "Quit")))

(fn `AsteroidCounter`
  (params (AsteroidDestroyed :type Integer))
  (set `self.AsteroidCount` (+ AsteroidDestroyed (`self.AsteroidCount`))))

(fn `GetAsteroidScore`
  (returns (Score :type Integer))
  ;[1 1 1] Return Asteroid count
  (return (`self.AsteroidCount`)))

(fn `UserConstructionScript`)