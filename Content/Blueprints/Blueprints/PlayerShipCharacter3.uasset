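; Red-tinted player ship character for a 2D space game on the X-Z plane, firing photon torpedoes on the FirePlayer2 input.
; Axis inputs apply impulses and set facing, while Tick applies that rotation and adds a spring-like pull toward player character 0.
; BeginPlay gives a random vertical kick.
; Asteroid hits or torpedo overlaps hide the ship, destroy the other actor and restart the level after a delay.
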(event `self.ReceiveActorBeginOverlap`
  (params (OtherActor :type "Actor Object Reference")))

(event `self.CapsuleComponent.OnComponentHit`
  (params (OtherActor :type "Actor Object Reference") (OtherComp :type "PrimitiveComponent Object Reference") (NormalImpulse :type "Vector Structure") (Hit :type "HitResult Structure (by ref)"))
  ;[1 1 1] Restart the level when an asteroid hits the player
  (bind _asasteroid_base (cast `/Game/Blueprints/AsteroidBase` OtherActor))
  (`self.SetActorHiddenInGame` true)
  (`self.K2_DestroyActor` _asasteroid_base)
  (`KismetSystemLibrary.Delay` 2.0)
  (`GameplayStatics.OpenLevel` (`self.CurrentLevelName`)))

(event `self.CapsuleComponent.OnComponentBeginOverlap`
  (params (OtherActor :type "Actor Object Reference") (OtherComp :type "PrimitiveComponent Object Reference") (OtherBodyIndex :type Integer) (bFromSweep :type Boolean) (SweepResult :type "HitResult Structure (by ref)"))
  ;[1 1 1] Restart the level when a torpedo hits the player
  (bind _asphoton_torpedo (cast `/Game/Blueprints/PhotonTorpedo` OtherActor))
  (`self.SetActorHiddenInGame` true)
  (`self.K2_DestroyActor` _asphoton_torpedo)
  (`KismetSystemLibrary.Delay` 2.0)
  (`GameplayStatics.OpenLevel` (`self.CurrentLevelName`)))

(event `/Game/Blueprints/Blueprints/PlayerShipCharacter2.ReceiveBeginPlay`
  (`PrimitiveComponent.AddImpulse` (`MovementComponent.UpdatedPrimitive` (`self.CharacterMovement`)) (* (`KismetMathLibrary.MakeVector` 0.0 0.0 (`KismetMathLibrary.RandomFloatInRange` -1.0 1.0)) 500.0) "None" true)
  (`PaperFlipbookComponent.SetSpriteColor` (`self.Sprite`) (struct :`R` 1.0 :`G` 0.08689 :`B` 0.115543 :`A` 1.0))
  (bind _returnvalue (`GameplayStatics.GetCurrentLevelName` true))
  (set `self.CurrentLevelName` (`KismetStringLibrary.Conv_StringToName` _returnvalue)))

(event `/Game/Blueprints/Blueprints/PlayerShipCharacter2.ReceiveTick`
  (params (DeltaSeconds :type "Float (single-precision)"))
  (bind _updatedprimitive (`MovementComponent.UpdatedPrimitive` (`self.CharacterMovement`)))
  ;[1 1 1] Movement
  (`self.SetActorRotation` (`self.ControlShipRotation`))
  (`PrimitiveComponent.AddImpulse` _updatedprimitive (`KismetMathLibrary.MakeVector` (+ (* 10.0 (stale `MoveRight` AxisValue)) (* (- (.x (`self.K2_GetActorLocation`)) (.x (`self.K2_GetActorLocation` (`GameplayStatics.GetPlayerCharacter` 0)))) -0.03)) 0.0 (+ (* 10.0 (stale `MoveUp` AxisValue)) (* (- (.z (`self.K2_GetActorLocation`)) (.z (`self.K2_GetActorLocation` (`GameplayStatics.GetPlayerCharacter` 0)))) -0.03))) "None" true)
  (`PrimitiveComponent.AddImpulse` _updatedprimitive (0.0 0.0 0.0) "None" true))

(event `MoveRight`
  (params (AxisValue :type "Float (double-precision)"))
  (bind _returnvalue (* AxisValue -90.0))
  ;[1 1 1] Movement
  (`PrimitiveComponent.AddImpulse` (`MovementComponent.UpdatedPrimitive` (`self.CharacterMovement`)) (`KismetMathLibrary.MakeVector` (* 10.0 AxisValue)) "None" true)
  (if (> (`KismetMathLibrary.Abs` _returnvalue) 45.0)
    (set `self.ControlShipRotation` (`KismetMathLibrary.MakeRotator` 0.0 (+ _returnvalue 90.0)))))

(event `MoveUp`
  (params (AxisValue :type "Float (double-precision)"))
  (bind _returnvalue (* AxisValue 90.0))
  ;[1 1 1] Movement
  (`PrimitiveComponent.AddImpulse` (`MovementComponent.UpdatedPrimitive` (`self.CharacterMovement`)) (`KismetMathLibrary.MakeVector` 0.0 0.0 (* 10.0 AxisValue)) "None" true)
  (if (> (`KismetMathLibrary.Abs` _returnvalue) 45.0)
    (set `self.ControlShipRotation` (`KismetMathLibrary.MakeRotator` 0.0 _returnvalue))))

(event `FirePlayer2`
  (bind _returnvalue (`self.GetActorForwardVector`))
  ;[1 1 1] Fire a Photon Torpedo
  (bind _returnvalue_2 (`|SpawnActorFromClass` "/Game/Blueprints/PhotonTorpedo.PhotonTorpedo_C" (`KismetMathLibrary.MakeTransform` (+ (* _returnvalue 75.0) (`self.K2_GetActorLocation`)) (`KismetMathLibrary.MakeRotator` 0.0 (+ (.pitch (`self.ControlShipRotation`)) -90.0))) "Undefined" "OverrideRootScale"))
  (`/Game/Blueprints/PhotonTorpedo.SetVelocity` _returnvalue_2 (* _returnvalue (`self.TorpedoSpeed`))))

(fn `UserConstructionScript`)