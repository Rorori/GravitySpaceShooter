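; Spawner actor that continuously emits moving asteroids from BeginPlay onward.
; A self-retriggering event spawns one, waits SpawnDelay, then repeats.
; Each spawn keeps the spawner's Y and Z, offsetting X randomly between the left and right spawn bounds.
; SpawnAsteroid creates the configured AsteroidType, casts it to AsteroidBase, and sets its velocity from the X/Z direction variables scaled by AsteroidSpeed.
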(event `OnSpawnAsteroid`
  ;[1 1 1] Spawn an asteroid, wait, then spawn another
  (`self.SpawnAsteroid` (`KismetMathLibrary.MakeVector` (+ (.x (`self.K2_GetActorLocation`)) (`KismetMathLibrary.RandomFloatInRange` (.x (`self.LeftSpawnLocation`)) (.x (`self.RightSpawnLocation`)))) (.y (`self.K2_GetActorLocation`)) (.z (`self.K2_GetActorLocation`))))
  (`KismetSystemLibrary.Delay` (`self.SpawnDelay`))
  (`self.OnSpawnAsteroid`) ; Trigger spawn event again. This creates a loop
)

(event `self.ReceiveBeginPlay`
  ;[1 1 1] Spawn an asteroid as soon as play begins
  (`self.OnSpawnAsteroid`))

(event `self.ReceiveActorBeginOverlap`
  (params (OtherActor :type "Actor Object Reference")))

(event `self.ReceiveTick`
  (params (DeltaSeconds :type "Float (single-precision)")))

(fn `SpawnAsteroid`
  (params (SpawnLocation :type "Vector Structure"))
  ;[1 1 1] Comment
  (bind _returnvalue (`|SpawnActorFromClass` (`self.AsteroidType`) (`KismetMathLibrary.MakeTransform` SpawnLocation) "Undefined" "OverrideRootScale")) ; spawn an asteroid. Use the class stored in AsteroidType to specify the kind of asteroid
  (bind _asasteroid_base (cast `/Game/Blueprints/AsteroidBase` _returnvalue)) ; Since we're not sure which type of asteroid we have, cast object to base class which has a SetVelocity method that we can use to set the speed of the asteroid.
  (`/Game/Blueprints/AsteroidBase.SetVelocity` _asasteroid_base (* (`KismetMathLibrary.MakeVector` (`self.LeftRightSpawnDirection`) 0.0 (`self.UpDownSpawnDirection`)) (`self.AsteroidSpeed`))))

(fn `UserConstructionScript`)